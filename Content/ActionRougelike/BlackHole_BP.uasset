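; Black hole actor that pulls in and destroys physics objects over a five-second lifespan.
; On BeginPlay, a timeline grows the radial force radius, strengthens its negative impulse and expands the sphere collision.
; Tick fires the radial impulse every frame to draw bodies inward.
; Any actor whose overlapping component simulates physics is destroyed when it enters the sphere.
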(event `self.ReceiveBeginPlay`
  (bind _radialforce (`self.RadialForce`))
  (`|ExecutionSequence`
    (:`then_1`
      (`self.SetLifeSpan` 5.0))
    (:`then_2`
      (bind (_direction _lerp_1 _lerp2 _lerp3) (`Timeline|RangeGrowth` :!via `PlayFromStart`)
        (:`Update`
          (`|ExecutionSequence`
            (:`then_0`
              (set `RadialForceComponent.Radius` (`KismetMathLibrary.Lerp` 50.0 (`self.MaxRange`) _lerp_1) _radialforce))
            (:`then_1`
              (set `RadialForceComponent.ImpulseStrength` (`KismetMathLibrary.Lerp` -250.0 -1000.0 _lerp2) _radialforce))
            (:`then_2`
              (`SphereComponent.SetSphereRadius` (`self.SphereComp`) (`KismetMathLibrary.Lerp` 40.0 500.0 _lerp3) true))))))))

(event `self.ReceiveTick`
  (params (DeltaSeconds :type "Float (single-precision)"))
  (`RadialForceComponent.FireImpulse` (`self.RadialForce`)))

(event `self.SphereComp.OnComponentBeginOverlap`
  (params (OverlappedComponent :type "PrimitiveComponent Object Reference") (OtherActor :type "Actor Object Reference") (OtherComp :type "PrimitiveComponent Object Reference") (OtherBodyIndex :type Integer) (bFromSweep :type Boolean) (SweepResult :type "HitResult Structure (by ref)"))
  (if (`SceneComponent.IsSimulatingPhysics` OtherComp "None")
    (`self.K2_DestroyActor` OtherActor)))

(fn `NewFunction`)

(fn `UserConstructionScript`)